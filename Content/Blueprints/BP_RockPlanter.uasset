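; BP_RockPlanter is a pickup item that lets the third-person character plant trees.
; On overlap it stores the character and passes itself to the character's PickUpItem.
; PickUp attaches it to the right-hand grip socket, halves the sphere mesh scale and disables that mesh's collision.
; PrimaryAction spawns a BP_Tree just below the player's location, while Drop destroys the planter.
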(event EventDrop
  (Development|PrintText "This rock planter has been dropped")
  (Actor|DestroyActor))

(event EventPrimaryAction
  (bind _player (Variables|Default|GetPlayer))
  (bind _returnvalue (Transformation|GetActorTransform _player))
  (Development|PrintText "Rock planted")
  (Game|SpawnActorfromClass "/Game/Blueprints/BP_Tree.BP_Tree_C" (Math|Transform|MakeTransform (+ (.location _returnvalue) "0.000000,0.000000,-100.000000") (.rotation _returnvalue) "1.000000,1.000000,1.000000") "Undefined" "MultiplyWithRoot" 0 0))

(event EventPickUp
  (bind _spheremesh (Variables|Default|GetSphereMesh))
  (Development|PrintText "This rock planter has been picked up")
  (Transformation|AttachComponentToComponent (Variables|/Script/Engine.Character|GetMesh (Variables|Default|GetPlayer)) "HandGrip_R" "SnapToTarget" "SnapToTarget" "KeepRelative" true)
  (Transformation|SetRelativeScale3D _spheremesh (/ (Variables|/Script/Engine.SceneComponent|GetRelativeScale3D _spheremesh) 2))
  (Collision|SetCollisionEnabled _spheremesh "NoCollision"))

(event Collision|EventActorBeginOverlap
  (params (OtherActor :type Actor%20Object%20Reference))
  (bind _asbp_third_person_character (Utilities|Casting|CastToBP_ThirdPersonCharacter OtherActor))
  (bind _output_get (Variables|Default|SetPlayer _asbp_third_person_character))
  (Default|PickUpItem _output_get self))

(fn ConstructionScript)