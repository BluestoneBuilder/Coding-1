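; BP_Tree is a tree actor that grows larger in random steps after it spawns.
; BeginPlay runs a latent loop that waits a random few seconds, adds a random uniform increment to TreeMesh's relative scale and decrements GrowCounter.
; The Delay wires back into the counter check, so growth stops without Tick once GrowCounter is no longer positive.
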(event EventBeginPlay
  (bind _tree_mesh (Variables|Default|GetTree%20Mesh))
  (if (> (Variables|Default|GetGrowCounter) 0) :!label _label
    ;[0.15 0.15 0.15 0.5] Tree grow loop
    (Utilities|FlowControl|Delay (Math|Random|RandomFloatinRange 4.0 6.0))
    (Transformation|SetRelativeScale3D _tree_mesh (+ (Variables|/Script/Engine.SceneComponent|GetRelativeScale3D _tree_mesh) (Math|Random|RandomFloatinRange 0.2 0.4)))
    (Math|Integer|DecrementInt (Variables|Default|GetGrowCounter)
      (:%20%20
        (goto _label)))))

(event Collision|EventActorBeginOverlap
  (params (OtherActor :type Actor%20Object%20Reference)))

(event EventTick
  (params (DeltaSeconds :type Float%20%28single-precision%29)))

(fn ConstructionScript)