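; BP_Camera is a security camera that signals detection of the third-person character through its spotlight color.
; When MovingCamera is set, a timeline sweeps the camera mesh's yaw between negative and positive RotationAmount.
; Overlap with an unobstructed visibility trace switches the light to a second color, then a repeat check after SpottingTime switches it to a third.
; Ending the overlap clears IsInView and restores the first color.
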(event Custom|Set%20Light%20Color
  (params (ColorIndex :type Integer))
  (Rendering|Components|Light|SetLightColor (Variables|Default|GetSpotLight) (Math|Conversions|ToLinearColor(Color) (Utilities|Array|Get(acopy) (Variables|Default|GetLightColors) ColorIndex)) true))

(event EventBeginPlay
  (bind _rotationamount (Variables|Default|GetRotationAmount))
  ;[0.01364 0.15 0.06485 0.5] CameraMovement
  (CallFunction|SetLightColor)
  (if (Variables|Default|GetMovingCamera)
    (bind _rotation_track (Timeline|CameraRotation Play)
      (:Update
        (Transformation|SetRelativeRotation (Variables|Default|GetSM_Security_Camera) (Math|Rotator|MakeRotator 0.0 0.0 (Math|Float|Lerp (* _rotationamount -1.0) _rotationamount _rotation_track)) false false)))))

(event Collision|EventActorBeginOverlap
  (params (OtherActor :type Actor%20Object%20Reference))
  (bind _spotlight (Variables|Default|GetSpotLight))
  (bind _returnvalue (Transformation|GetWorldLocation _spotlight))
  ;[0.15 0 0 0.5] CameraDetection
  (bind _asbp_third_person_character (Utilities|Casting|CastToBP_ThirdPersonCharacter OtherActor))
  (bind _returnvalue_2 (Collision|LineTraceByChannel _returnvalue (Transformation|GetActorLocation _asbp_third_person_character) "TraceTypeQuery1" false 0 "ForDuration"))
  (if (not _returnvalue_2)
    (Variables|Default|SetisInView true)
    (CallFunction|SetLightColor 1)
    (Utilities|FlowControl|Delay (Variables|Default|GetSpottingTime))
    (if (Variables|Default|GetisInView)
      (bind _returnvalue_3 (Collision|LineTraceByChannel _returnvalue (Transformation|GetActorLocation _asbp_third_person_character) "TraceTypeQuery1" false 0 "ForDuration"))
      (if (not _returnvalue_3)
        (CallFunction|SetLightColor 2)))))

(event Collision|EventActorEndOverlap
  (params (OtherActor :type Actor%20Object%20Reference))
  ;[0.15 0 0 0.5] CameraDetection
  (Utilities|Casting|CastToBP_ThirdPersonCharacter OtherActor)
  (Variables|Default|SetisInView false)
  (CallFunction|SetLightColor))

(fn ConstructionScript)