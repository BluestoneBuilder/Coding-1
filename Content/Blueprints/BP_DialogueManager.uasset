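; BP_DialogueManager is a simple Blueprint that shows dialogue lines one at a time.
; Each DisplayNextLine call prints the current entry of the Dialogue array as text for a few seconds, then advances the Index.
; The Index wraps to the start once it passes the last line, so the dialogue cycles endlessly.
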(event Custom|DisplayNextLine
  (if (>= (Variables|Default|GetIndex) (Utilities|Array|Length (Variables|Default|GetDialogue)))
    (Variables|Default|SetIndex 0))
  (Development|PrintText (Utilities|Array|Get(acopy) (Variables|Default|GetDialogue) (Variables|Default|GetIndex)) true true "(R=0.000000,G=0.660000,B=1.000000,A=1.000000)" 5.0)
  (Math|Integer|IncrementInt (Variables|Default|GetIndex)))

(fn ConstructionScript)