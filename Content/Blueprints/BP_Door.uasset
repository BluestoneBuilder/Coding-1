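; BP_Door is a security-gated door that swings open when the third-person player character overlaps it.
; On overlap, a closed door compares the character's SecurityLevel to RequiredSecurityLevel, then either prints an unlock message and plays the SwingDoorOpen timeline or prints the required level.
; The timeline's float drives a yaw Lerp on the door mesh.
; End overlap clears IsOpen and reverses the timeline to close it.
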(event EventBeginPlay)

(event Collision|EventActorBeginOverlap
  (params (OtherActor :type Actor%20Object%20Reference))
  (bind _requiredsecuritylevel (Variables|Default|GetrequiredSecurityLevel))
  (bind _asbp_third_person_character (Utilities|Casting|CastToBP_ThirdPersonCharacter OtherActor)) ; Is this the player
  (if (not (Variables|Default|GetisOpen))
    (if (>= (Variables|/Game/ThirdPerson/Blueprints/BP_ThirdPersonCharacter.BP_ThirdPersonCharacter_C|GetsecurityLevel _asbp_third_person_character) _requiredsecuritylevel)
      (Variables|Default|SetisOpen true)
      (Development|PrintText "Unlocking door.")
      (bind _rotationfloat (Timeline|Swing%20Door%20Open Play)
        (:Update
          (Transformation|SetRelativeRotation (Variables|Default|GetSM_FrontDoor_A_Door) (Math|Rotator|MakeRotator 0.0 0.0 (Math|Float|Lerp 0.0 -1.3e+02 _rotationfloat)) false false)))
      (else
        (Development|PrintText (Utilities|Text|FormatText "Security level {Security Level} required." _requiredsecuritylevel))))))

(event EventTick
  (params (DeltaSeconds :type Float%20%28single-precision%29)))

(event Collision|EventActorEndOverlap
  (params (OtherActor :type Actor%20Object%20Reference))
  (Utilities|Casting|CastToBP_ThirdPersonCharacter OtherActor)
  (Variables|Default|SetisOpen false)
  (bind _rotationfloat (Timeline|Swing%20Door%20Open Reverse)
    (:Update
      (Transformation|SetRelativeRotation (Variables|Default|GetSM_FrontDoor_A_Door) (Math|Rotator|MakeRotator 0.0 0.0 (Math|Float|Lerp 0.0 -1.3e+02 _rotationfloat)) false false))))

(fn ConstructionScript)