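; BP_LoopsAndLists is a Blueprint that demonstrates while loops, for-each loops and array indexing with on-screen text.
; After a short delay, BeginPlay counts WhileCounter down to zero, printing each number in a color picked from Colors by modulo 7.
; In parallel, AdjustKeysJump raises every BP_Keycard actor, prints how many moved, then re-calls itself each second, so the keycards climb indefinitely.
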(event Custom|AdjustKeysJump
  (bind _outactors (Actor|GetAllActorsOfClass "/Game/Blueprints/BP_Keycard.BP_Keycard_C"))
  (for _array_element _outactors
    (Transformation|AddRelativeLocation (Variables|/Game/Blueprints/BP_Keycard.BP_Keycard_C|GetDefaultSceneRoot _array_element) "0.000000,0.000000,50.000000" false false))
  (Development|PrintText (Utilities|Text|FormatText "We have raised {count} keycards." (Utilities|Array|Length _outactors)) true true "(R=0.000000,G=0.660000,B=1.000000,A=1.000000)" 1e+01)
  (Utilities|FlowControl|Delay 1.0)
  (CallFunction|AdjustKeysJump))

(event EventBeginPlay
  (bind _whilecounter (Variables|Default|GetWhileCounter))
  (Utilities|FlowControl|Sequence
    (:then_0
      ;[0.15 0.15 0.15 0.5] Comment
      (Utilities|FlowControl|Delay 2.0)
      (while (> _whilecounter 0)
        (Development|PrintText (Utilities|Text|FormatText "We are in loop number {count}" _whilecounter) true true (Utilities|Array|Get(acopy) (Variables|Default|GetColors) (Math|Integer|%(Integer) (Variables|Default|GetWhileCounter) 7)))
        (Math|Integer|DecrementInt _whilecounter)))
    (:then_1
      (Utilities|FlowControl|Delay 0.2)
      (CallFunction|AdjustKeysJump))))

(fn ConstructionScript)